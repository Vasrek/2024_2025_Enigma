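; BP_MainMenu is a main menu pawn that shows the menu widget and routes Enhanced Input navigation to it.
; On BeginPlay it adds the IMC_MainMenu mapping context, creates WBP_MainMenu, shows the mouse cursor and sets Game and UI input focused on the widget.
; The Up, Down and Select input actions call the widget's GoUp, GoDown and Select functions, each printing a debug string first.
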(event `self.ReceiveBeginPlay`
  (bind _returnvalue (`GameplayStatics.GetPlayerController` 0))
  (bind _returnvalue_2 (pcsubsystem `EnhancedInputLocalPlayerSubsystem` (`GameplayStatics.GetPlayerController` 0)))
  (`/Engine/EditorBlueprintResources/StandardMacros.IsValid` _returnvalue_2
    (:`Is Valid`
      (`EnhancedInputSubsystemInterface.AddMappingContext` _returnvalue_2 "/Game/01-Blueprints/Inputs/IMC_MainMenu.IMC_MainMenu" 0 (struct))
      (bind _returnvalue_3 (`|CreateWidget` "/Game/01-Blueprints/Widgets/WBP_MainMenu.WBP_MainMenu_C"))
      (bind _output_get (set `self.WBPMainMenuRef` _returnvalue_3))
      (`UserWidget.AddToViewport` _output_get 0)
      (set `PlayerController.bShowMouseCursor` true _returnvalue)
      (`WidgetBlueprintLibrary.SetInputMode_GameAndUIEx` _returnvalue (`self.WBPMainMenuRef`)))))

(event `EnhancedInput|/Game/01-Blueprints/Inputs/Actions/MainMenu/IA_Up`
  (params (ActionValue :type Boolean) (ElapsedSeconds :type "Float (double-precision)") (TriggeredSeconds :type "Float (double-precision)") (InputAction :type "InputAction Object Reference" :default "/Game/01-Blueprints/Inputs/Actions/MainMenu/IA_Up.IA_Up"))
  (:`Started`
    (`KismetSystemLibrary.PrintString` "UP")
    (`/Game/01-Blueprints/Widgets/WBP_MainMenu.GoUp` (`self.WBPMainMenuRef`))))

(event `EnhancedInput|/Game/01-Blueprints/Inputs/Actions/MainMenu/IA_Down`
  (params (ActionValue :type Boolean) (ElapsedSeconds :type "Float (double-precision)") (TriggeredSeconds :type "Float (double-precision)") (InputAction :type "InputAction Object Reference" :default "/Game/01-Blueprints/Inputs/Actions/MainMenu/IA_Down.IA_Down"))
  (:`Started`
    (`KismetSystemLibrary.PrintString` "DOWN")
    (`/Game/01-Blueprints/Widgets/WBP_MainMenu.GoDown` (`self.WBPMainMenuRef`))))

(event `EnhancedInput|/Game/01-Blueprints/Inputs/Actions/MainMenu/IA_Select`
  (params (ActionValue :type Boolean) (ElapsedSeconds :type "Float (double-precision)") (TriggeredSeconds :type "Float (double-precision)") (InputAction :type "InputAction Object Reference" :default "/Game/01-Blueprints/Inputs/Actions/MainMenu/IA_Select.IA_Select"))
  (:`Started`
    (`KismetSystemLibrary.PrintString` "SELECT")
    (`/Game/01-Blueprints/Widgets/WBP_MainMenu.Select` (`self.WBPMainMenuRef`))))

(fn `UserConstructionScript`)