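; BP_Player is the player character, handling Enhanced Input move, look and jump, plus gold collection and respawning.
; BeginPlay records the spawn transform, creates the HUD and caches GI_Game; Death teleports the player back to that transform.
; AddGold updates the running total and HUD.
; Pressing J saves gold as BestScore to the save slot and game instance if it beats the record, then opens the main menu after a short delay.
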(event `self.ReceiveBeginPlay`
  (bind _returnvalue (`GameplayStatics.GetPlayerController` 0))
  (bind _returnvalue_2 (`GameplayStatics.GetPlayerController` 0))
  (`/Engine/EditorBlueprintResources/StandardMacros.IsValid` _returnvalue
    (:`Is Valid`
      (`EnhancedInputSubsystemInterface.AddMappingContext` (pcsubsystem `EnhancedInputLocalPlayerSubsystem` _returnvalue) "/Game/01-Blueprints/Inputs/IMC_Player.IMC_Player" 0 (struct))
      (set `self.RespawnTransform` (`self.GetTransform`))
      (set `PlayerController.bShowMouseCursor` false _returnvalue_2)
      (`WidgetBlueprintLibrary.SetInputMode_GameOnly` _returnvalue_2)
      (bind _returnvalue_3 (`|CreateWidget` "/Game/01-Blueprints/Widgets/WBP_HUD.WBP_HUD_C"))
      (bind _output_get (set `self.HUDRef` _returnvalue_3))
      (`UserWidget.AddToViewport` _output_get 0)
      (bind _asgi_game (cast `/Game/01-Blueprints/GI_Game` (`GameplayStatics.GetGameInstance`)))
      (set `self.GameInstanceRef` _asgi_game))))

(event `EnhancedInput|/Game/01-Blueprints/Inputs/Actions/Player/IA_Player_Move`
  (params (ActionValue :type "Vector2D Structure") (ElapsedSeconds :type "Float (double-precision)") (TriggeredSeconds :type "Float (double-precision)") (InputAction :type "InputAction Object Reference" :default "/Game/01-Blueprints/Inputs/Actions/Player/IA_Player_Move.IA_Player_Move"))
  (bind (_returnvalue_roll _returnvalue_pitch _returnvalue_yaw) (`KismetMathLibrary.BreakRotator` (`self.GetControlRotation`)))
  (bind (_returnvalue_roll_2 _returnvalue_pitch_2 _returnvalue_yaw_2) (`KismetMathLibrary.BreakRotator` (`self.GetControlRotation`)))
  (:`Triggered`
    (`self.AddMovementInput` (`KismetMathLibrary.GetRightVector` (`KismetMathLibrary.MakeRotator` 0.0 0.0 _returnvalue_yaw_2)) ActionValue_X)
    (`self.AddMovementInput` (`KismetMathLibrary.GetForwardVector` (`KismetMathLibrary.MakeRotator` 0.0 0.0 _returnvalue_yaw)) ActionValue_Y)))

(event `EnhancedInput|/Game/01-Blueprints/Inputs/Actions/Player/IA_Player_Look`
  (params (ActionValue :type "Vector2D Structure") (ElapsedSeconds :type "Float (double-precision)") (TriggeredSeconds :type "Float (double-precision)") (InputAction :type "InputAction Object Reference" :default "/Game/01-Blueprints/Inputs/Actions/Player/IA_Player_Look.IA_Player_Look"))
  (:`Triggered`
    (`self.AddControllerYawInput` ActionValue_X)
    (`self.AddControllerPitchInput` ActionValue_Y)))

(event `EnhancedInput|/Game/01-Blueprints/Inputs/Actions/Player/IA_Player_Jump`
  (params (ActionValue :type Boolean) (ElapsedSeconds :type "Float (double-precision)") (TriggeredSeconds :type "Float (double-precision)") (InputAction :type "InputAction Object Reference" :default "/Game/01-Blueprints/Inputs/Actions/Player/IA_Player_Jump.IA_Player_Jump"))
  (:`Started`
    (`self.Jump`))
  (:`Completed`
    (`self.StopJumping`)))

(event `Death`
  (`self.K2_SetActorTransform` (`self.RespawnTransform`) false true))

(event `AddGold`
  (params (GoldsToAdd :type Integer))
  (bind _output_get (set `self.CurrentGold` (+ GoldsToAdd (`self.CurrentGold`))))
  (`/Game/01-Blueprints/Widgets/WBP_HUD.UpdateTXTGold` (`self.HUDRef`) _output_get))

(event `Key|J`
  (params (Key :type "Key Structure"))
  (:`Pressed`
    (if (> (`self.CurrentGold`) (`/Game/01-Blueprints/GI_Game.BestScore` (`self.GameInstanceRef`)))
      (bind _returnvalue (`GameplayStatics.DoesSaveGameExist` "BestScore"))
      (if _returnvalue
        (bind _returnvalue_2 (`GameplayStatics.LoadGameFromSlot` "BestScore"))
        (bind _assg_best_score (cast `/Game/01-Blueprints/SG_BestScore` _returnvalue_2))
        (set `/Game/01-Blueprints/SG_BestScore.BestScore` (`self.CurrentGold`) _assg_best_score)
        (`GameplayStatics.SaveGameToSlot` _assg_best_score "BestScore")
        (else
          (bind _returnvalue_3 (`GameplayStatics.CreateSaveGameObject` "/Game/01-Blueprints/SG_BestScore.SG_BestScore_C"))
          (set `/Game/01-Blueprints/SG_BestScore.BestScore` (`self.CurrentGold`) _returnvalue_3)
          (`GameplayStatics.SaveGameToSlot` _returnvalue_3 "BestScore")))
      (set `/Game/01-Blueprints/GI_Game.BestScore` (`self.CurrentGold`) (`self.GameInstanceRef`)))
    (`KismetSystemLibrary.Delay` 0.2)
    (`GameplayStatics.OpenLevelBySoftObjectPtr` "/Game/02-Levels/L_MainMenu.L_MainMenu")))

(fn `UserConstructionScript`)